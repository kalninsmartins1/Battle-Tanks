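; Tank Blueprint that provides camera aim controls and sets up the tank's barrel and turret references.
; The AimElevation axis pitches the SpringArm and AimAzimuth yaws a separate gimbal component, each adding scaled local rotation to keep the two camera axes on different components.
; On BeginPlay it passes the Barrel and TankTurret components to setter functions, with no aiming or firing logic in the graph itself.
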(event EventBeginPlay
  (Class|Tank|SetBarrelComponent (Variables|Default|GetBarrel))
  (Class|Tank|SetTurretComponent (Variables|Default|GetTankTurret)))

(event EventTick
  (params (DeltaSeconds :type Float%20%28single-precision%29)))

(event Input|AxisEvents|InputAxisAimAzimuth
  (params (AxisValue :type Float%20%28single-precision%29))
  ;[1 1 1] Move camera left and right
  (Transformation|AddLocalRotation (Variables|Default|GetAzimuth%20Gibal) (Math|Rotator|MakeRotator 0.0 0.0 (* AxisValue 5.0)) false false))

(event Input|AxisEvents|InputAxisAimElevation
  (params (AxisValue :type Float%20%28single-precision%29))
  ;[1 1 1] Move camera up and down
  (Transformation|AddLocalRotation (Variables|Default|GetSpringArm) (Math|Rotator|MakeRotator 0.0 (* AxisValue 5.0) 0.0) false false))

(fn ConstructionScript)